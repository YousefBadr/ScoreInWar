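; Turret Blueprint that hands its barrel, dome and projectile class to a TurretAiming component when play begins.
; BeginPlay calls Initialise on TurretAiming once that component, Barel and Dome are all valid, passing BP_Projectile as the projectile.
; If any reference is invalid, it waits briefly and retries the check through a DoN node that caps the number of attempts.
; The construction script is empty.
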(event EventBeginPlay
  (bind _turretaiming (Variables|Default|GetTurretAiming))
  (bind _dome (Variables|Default|GetDome))
  (bind _barel (Variables|Default|GetBarel))
  (if (Math|Boolean|ANDBoolean (Utilities|IsValid _turretaiming) (Utilities|IsValid _barel) (Utilities|IsValid _dome)) :!label _label
    (Class|TurretAimingComponent|Initialise _turretaiming _barel _dome "/Game/Projectile/BP_Projectile.BP_Projectile_C")
    (else
      (Utilities|FlowControl|Delay 2.0)
      (Utilities|FlowControl|DoN 10
        (:Exit
          (goto _label))))))

(fn ConstructionScript)