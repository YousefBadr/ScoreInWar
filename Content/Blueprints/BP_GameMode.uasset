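; Game mode Blueprint that sets up the main UI and background battle music.
; InitializeGame creates WBP_MainUI for the first player controller, adds it to the viewport, then spawns and activates a 2D music track stored in BackgroundAudio.
; StopSound deactivates that audio component.
; Calls to the RemoveLoadingWidget and ShowInGameWidget dispatchers are present but unconnected, so they never run.
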(event Custom|StopSound
  (Components|Activation|SetActive (Variables|Default|GetBackgroundAudio) false false))

(event EventInitializeGame
  (bind _returnvalue (UserInterface|CreateWidget "/Game/Blueprints/WBP_MainUI.WBP_MainUI_C" (Game|GetPlayerController 0)))
  (UserInterface|Viewport|AddtoViewport _returnvalue 0)
  (bind _returnvalue_2 (Audio|SpawnSound2D "/Game/Sounds/Jahzzar_-_Battle_Cue.Jahzzar_-_Battle_Cue" 1.0 1.0 0.0 0))
  (bind _output_get (Variables|Default|SetBackgroundAudio _returnvalue_2))
  (Components|Activation|SetActive _output_get true false))

(fn ConstructionScript)